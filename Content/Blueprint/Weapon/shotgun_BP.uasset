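; Shotgun weapon Blueprint that sets its clip, timing and HUD icon data and overrides parent weapon functions for firing, reloading and switching.
; Fire traces from the player's TPS camera, spawns a ShotgunAmmo_BP from the Arrow aimed at the impact point, passes on damage, then plays shell particles and animation.
; Reload animates and refills the clip, Switch stops animation, and Pickup and Drop toggle pickup-box collision.
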(event `self.ReceiveBeginPlay`
  (set `self.Clip` 12)
  (set `self.MaxClipSize` 12)
  (set `self.ReloadTime` 4.3)
  (set `self.FireRate` 1.0)
  (set `self.weaponType` "shotgun")
  (set `self.WeaponIcon` "/Game/UI/shotgunIcon.shotgunIcon"))

(event `/Game/Blueprint/PickupSystem/PickupWeapon_BPInterface.Pickup`
  (`PrimitiveComponent.SetCollisionEnabled` (`self.Shotgun_A`) "NoCollision")
  (`PrimitiveComponent.SetCollisionEnabled` (`self.Box`) "NoCollision"))

(event `/Game/Blueprint/PickupSystem/PickupWeapon_BPInterface.Drop`
  (`PrimitiveComponent.SetCollisionEnabled` (`self.Shotgun_A`) "NoCollision")
  (`PrimitiveComponent.SetCollisionEnabled` (`self.Box`) "QueryOnly"))

(fn `Fire`
  (bind _returnvalue (`SceneComponent.K2_GetComponentLocation` (`self.Arrow`)))
  (`parent.Fire`)
  (bind _asmannequin_bp (cast `/Game/Blueprint/Mannequin/mannequinBP` (`GameplayStatics.GetPlayerCharacter` 0)))
  (bind _tpscamera (`/Game/Blueprint/Mannequin/mannequinBP.TPSCamera` _asmannequin_bp))
  (bind _returnvalue_2 (`SceneComponent.K2_GetComponentLocation` _tpscamera))
  (bind _outhit (`KismetSystemLibrary.LineTraceSingle` _returnvalue_2 (+ _returnvalue_2 (* (`SceneComponent.GetForwardVector` _tpscamera) (8192.0 8192.0 8192.0))) "TraceTypeQuery1"))
  (bind _returnvalue_3 (`|SpawnActorFromClass` "/Game/Blueprint/Ammunition/shotgunAmmo_BP.shotgunAmmo_BP_C" (`KismetMathLibrary.MakeTransform` _returnvalue (`KismetMathLibrary.FindLookAtRotation` _returnvalue (`.ImpactPoint` (`GameplayStatics.BreakHitResult` _outhit)))) "AlwaysSpawn" "OverrideRootScale" self (`GameplayStatics.GetPlayerCharacter` 0)))
  (`/Game/Blueprint/Ammunition/BulletCollision.SetDamage` _returnvalue_3 (`self.WeaponDamage`))
  (`ActorComponent.Activate` (`self.ShotgunShellParticleSystem`) true)
  (set `self.Clip` (- (`self.Clip`) 1))
  (`SkeletalMeshComponent.PlayAnimation` (`self.Shotgun_A`) "/Game/Weapon_part1/MilitaryWeapSilver/Weapons/Animations/Fire_Shotgun_W.Fire_Shotgun_W" false))

(fn `GetPickupName`
  (returns (PickupName :type String))
  (return "shotgun"))

(fn `GetWeaponIconSize`
  (returns (ImageSize :type "Vector Structure") (Position :type "Vector Structure"))
  (`parent.GetWeaponIconSize`)
  (cast `Texture2D` (`self.WeaponIcon`))
  (return (`KismetMathLibrary.MakeVector` 200.0 200.0) (0.0 45.0 0.0)))

(fn `Reload`
  (params (nbBullet :type Integer))
  (`parent.Reload` 0)
  (`SkeletalMeshComponent.PlayAnimation` (`self.Shotgun_A`) "/Game/Weapon_part1/MilitaryWeapSilver/Weapons/Animations/Reload_Shotgun_Hip_W.Reload_Shotgun_Hip_W" false)
  (set `self.Clip` nbBullet))

(fn `Switch`
  (`parent.Switch`)
  (`SkeletalMeshComponent.Stop` (`self.Shotgun_A`)))

(fn `UserConstructionScript`)