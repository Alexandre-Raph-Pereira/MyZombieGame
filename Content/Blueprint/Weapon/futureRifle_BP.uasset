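; Rifle weapon Blueprint that extends a parent weapon class, setting its clip, fire rate, reload time and icon on BeginPlay.
; Fire traces from the player's third-person camera, then spawns a RifleAmmo_BP projectile at the muzzle arrow aimed at the impact point, passing on weapon damage.
; Fire and Reload update the clip and play mesh animations; Switch stops them.
; Pickup and Drop toggle the box's query collision.
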(event `self.ReceiveBeginPlay`
  (set `self.Clip` 15)
  (set `self.MaxClipSize` 15)
  (set `self.ReloadTime` 2.0)
  (set `self.FireRate` 0.5)
  (set `self.weaponType` "rifle")
  (set `self.WeaponIcon` "/Game/UI/ar4Icon-removebg-preview.ar4Icon-removebg-preview")
  (set `self.FireAnim` "/Game/Weapon_part1/MilitaryWeapSilver/Weapons/Animations/Fire_Pistol_W.Fire_Pistol_W"))

(event `/Game/Blueprint/PickupSystem/PickupWeapon_BPInterface.Pickup`
  (`PrimitiveComponent.SetCollisionEnabled` (`self.SM_Rifle`) "NoCollision")
  (`PrimitiveComponent.SetCollisionEnabled` (`self.Box`) "NoCollision"))

(event `/Game/Blueprint/PickupSystem/PickupWeapon_BPInterface.Drop`
  (`PrimitiveComponent.SetCollisionEnabled` (`self.SM_Rifle`) "NoCollision")
  (`PrimitiveComponent.SetCollisionEnabled` (`self.Box`) "QueryOnly"))

(fn `Fire`
  (bind _returnvalue (`SceneComponent.K2_GetComponentLocation` (`self.Arrow`)))
  (`parent.Fire`)
  (bind _asmannequin_bp (cast `/Game/Blueprint/Mannequin/mannequinBP` (`GameplayStatics.GetPlayerCharacter` 0)))
  (bind _tpscamera (`/Game/Blueprint/Mannequin/mannequinBP.TPSCamera` _asmannequin_bp))
  (bind _returnvalue_2 (`SceneComponent.K2_GetComponentLocation` _tpscamera))
  (bind _outhit (`KismetSystemLibrary.LineTraceSingle` _returnvalue_2 (+ _returnvalue_2 (* (`SceneComponent.GetForwardVector` _tpscamera) (8192.0 8192.0 8192.0))) "TraceTypeQuery1"))
  (bind _returnvalue_3 (`|SpawnActorFromClass` "/Game/Blueprint/Ammunition/rifleAmmo_BP.rifleAmmo_BP_C" (`KismetMathLibrary.MakeTransform` _returnvalue (`KismetMathLibrary.FindLookAtRotation` _returnvalue (`.ImpactPoint` (`GameplayStatics.BreakHitResult` _outhit)))) "AlwaysSpawn" "OverrideRootScale" self (`GameplayStatics.GetPlayerCharacter` 0)))
  (`/Game/Blueprint/Ammunition/BulletCollision.SetDamage` _returnvalue_3 (`self.WeaponDamage`))
  (`ActorComponent.Activate` (`self.NewParticleSystem`) true)
  (set `self.Clip` (- (`self.Clip`) 1))
  (`SkeletalMeshComponent.PlayAnimation` (`self.SM_Rifle`) "/Game/Weapons/Rifle/Animations/Weap_Rifle_Fire.Weap_Rifle_Fire" false))

(fn `GetPickupName`
  (returns (PickupName :type String))
  (return "rifle"))

(fn `GetWeaponIconSize`
  (returns (ImageSize :type "Vector Structure") (Position :type "Vector Structure"))
  (`parent.GetWeaponIconSize`)
  (bind _astexture_2d (cast `Texture2D` (`self.WeaponIcon`)))
  (return (`KismetMathLibrary.MakeVector` (/ (`KismetMathLibrary.Conv_IntToDouble` (`Texture2D.Blueprint_GetSizeX` _astexture_2d)) 4.0) (/ (`KismetMathLibrary.Conv_IntToDouble` (`Texture2D.Blueprint_GetSizeY` _astexture_2d)) 3.75)) (0.0 0.0 0.0)))

(fn `Reload`
  (params (nbBullet :type Integer))
  (`parent.Reload` 0)
  (`SkeletalMeshComponent.PlayAnimation` (`self.SM_Rifle`) "/Game/Weapons/Rifle/Animations/Weap_Rifle_Reload.Weap_Rifle_Reload" false)
  (set `self.Clip` nbBullet))

(fn `Switch`
  (`parent.Switch`)
  (`SkeletalMeshComponent.Stop` (`self.SM_Rifle`)))

(fn `UserConstructionScript`)