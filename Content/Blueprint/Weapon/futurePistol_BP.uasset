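; Pistol weapon Blueprint that extends a parent weapon with its own stats, icon, animations and pickup name.
; Fire traces from the player's third-person camera, then spawns a PistolAmmo_BP projectile at the Arrow aimed at the impact point, passing on damage.
; It also decrements the clip and plays shell particles and animation, while Reload sets the clip to the given count.
; Pickup and Drop toggle the Box collision.
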(event `self.ReceiveBeginPlay`
  (set `self.Clip` 15)
  (set `self.MaxClipSize` 15)
  (set `self.ReloadTime` 1.5)
  (set `self.FireRate` 0.6)
  (set `self.weaponType` "pistol")
  (set `self.WeaponIcon` "/Game/UI/pistolIcon.pistolIcon")
  (set `self.FireAnim` "/Game/Weapons/Pistol/Animations/Weap_Pistol_Fire.Weap_Pistol_Fire"))

(event `/Game/Blueprint/PickupSystem/PickupWeapon_BPInterface.Pickup`
  (`PrimitiveComponent.SetCollisionEnabled` (`self.pistol`) "NoCollision")
  (`PrimitiveComponent.SetCollisionEnabled` (`self.Box`) "NoCollision"))

(event `/Game/Blueprint/PickupSystem/PickupWeapon_BPInterface.Drop`
  (`PrimitiveComponent.SetCollisionEnabled` (`self.pistol`) "NoCollision")
  (`PrimitiveComponent.SetCollisionEnabled` (`self.Box`) "QueryOnly"))

(fn `Fire`
  (bind _returnvalue (`SceneComponent.K2_GetComponentLocation` (`self.Arrow`)))
  (`parent.Fire`)
  (bind _asmannequin_bp (cast `/Game/Blueprint/Mannequin/mannequinBP` (`GameplayStatics.GetPlayerCharacter` 0)))
  (bind _tpscamera (`/Game/Blueprint/Mannequin/mannequinBP.TPSCamera` _asmannequin_bp))
  (bind _returnvalue_2 (`SceneComponent.K2_GetComponentLocation` _tpscamera))
  (bind _outhit (`KismetSystemLibrary.LineTraceSingle` _returnvalue_2 (+ _returnvalue_2 (* (`SceneComponent.GetForwardVector` _tpscamera) (8192.0 8192.0 8192.0))) "TraceTypeQuery1"))
  (bind _returnvalue_3 (`|SpawnActorFromClass` "/Game/Blueprint/Ammunition/pistolAmmo_BP.pistolAmmo_BP_C" (`KismetMathLibrary.MakeTransform` _returnvalue (`KismetMathLibrary.FindLookAtRotation` _returnvalue (`.ImpactPoint` (`GameplayStatics.BreakHitResult` _outhit)))) "AlwaysSpawn" "OverrideRootScale" self (`GameplayStatics.GetPlayerCharacter` 0)))
  (`/Game/Blueprint/Ammunition/BulletCollision.SetDamage` _returnvalue_3 (`self.WeaponDamage`))
  (`ActorComponent.Activate` (`self.PistolShellParticleSystem`) true)
  (set `self.Clip` (- (`self.Clip`) 1))
  (`SkeletalMeshComponent.PlayAnimation` (`self.pistol`) "/Game/Weapons/Pistol/Animations/Weap_Pistol_Fire.Weap_Pistol_Fire" false))

(fn `GetPickupName`
  (returns (PickupName :type String))
  (return "pistol"))

(fn `GetWeaponIconSize`
  (returns (ImageSize :type "Vector Structure") (Position :type "Vector Structure"))
  (`parent.GetWeaponIconSize`)
  (cast `Texture2D` (`self.WeaponIcon`))
  (return (`KismetMathLibrary.MakeVector` 170.0 100.0) (0.0 0.0 0.0)))

(fn `Reload`
  (params (nbBullet :type Integer))
  (`parent.Reload` 0)
  (`SkeletalMeshComponent.PlayAnimation` (`self.pistol`) "/Game/Weapons/Pistol/Animations/Weap_Pistol_Reload.Weap_Pistol_Reload" false)
  (set `self.Clip` nbBullet))

(fn `Switch`
  (`parent.Switch`)
  (`SkeletalMeshComponent.Stop` (`self.pistol`)))

(fn `UserConstructionScript`)