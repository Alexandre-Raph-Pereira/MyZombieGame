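; Zombie enemy Blueprint that takes bullet damage and is destroyed when its health runs out.
; A Life component starts at a fixed health on BeginPlay, and separate head and body collision components detect hits from actors implementing the BulletCollision interface.
; Each hit reads damage through that interface, doubles it for headshots, and destroys the bullet.
; Capsule hits only print the other actor's name for debugging.
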(event `self.ReceiveBeginPlay`
  (`|VariableSetRef` (`.Life_5_FBD8569B49176CDD66AFA6B2A62CB2C6` (break `/Game/Blueprint/Life/CharacterLife_Structure` (`self.Life`))) 75))

(event `self.HeadCollision.OnComponentHit`
  (params (HitComponent :type "PrimitiveComponent Object Reference") (OtherActor :type "Actor Object Reference") (OtherComp :type "PrimitiveComponent Object Reference") (NormalImpulse :type "Vector Structure") (Hit :type "HitResult Structure (by ref)"))
  (bind _life (break `/Game/Blueprint/Life/CharacterLife_Structure` (`self.Life`)))
  ;[1 1 1] Head shot
  (if (`KismetSystemLibrary.DoesImplementInterface` OtherActor "/Game/Blueprint/Ammunition/BulletCollision.BulletCollision_C")
    (`KismetSystemLibrary.PrintString` "Head")
    (bind _damage (message `/Game/Blueprint/Ammunition/BulletCollision.GetDamage` OtherActor))
    (`|VariableSetRef` _life (- _life (* _damage 2)))
    (`self.K2_DestroyActor` OtherActor)
    (if (<= (`.Life_5_FBD8569B49176CDD66AFA6B2A62CB2C6` (break `/Game/Blueprint/Life/CharacterLife_Structure` (`self.Life`))) 0)
      (`/Game/Blueprint/Zombie/ZombieInterface.Die`))))

(event `self.BodyCollision.OnComponentHit`
  (params (HitComponent :type "PrimitiveComponent Object Reference") (OtherActor :type "Actor Object Reference") (OtherComp :type "PrimitiveComponent Object Reference") (NormalImpulse :type "Vector Structure") (Hit :type "HitResult Structure (by ref)"))
  (bind _life (break `/Game/Blueprint/Life/CharacterLife_Structure` (`self.Life`)))
  ;[1 1 1] Body shot
  (if (`KismetSystemLibrary.DoesImplementInterface` OtherActor "/Game/Blueprint/Ammunition/BulletCollision.BulletCollision_C")
    (`KismetSystemLibrary.PrintString` "Body")
    (bind _damage (message `/Game/Blueprint/Ammunition/BulletCollision.GetDamage` OtherActor))
    (`|VariableSetRef` _life (- _life _damage))
    (`self.K2_DestroyActor` OtherActor)
    (if (<= (`.Life_5_FBD8569B49176CDD66AFA6B2A62CB2C6` (break `/Game/Blueprint/Life/CharacterLife_Structure` (`self.Life`))) 0)
      (`/Game/Blueprint/Zombie/ZombieInterface.Die`))))

(event `/Game/Blueprint/Zombie/ZombieInterface.Die`
  (`self.K2_DestroyActor`))

(event `self.CapsuleComponent.OnComponentHit`
  (params (HitComponent :type "PrimitiveComponent Object Reference") (OtherActor :type "Actor Object Reference") (OtherComp :type "PrimitiveComponent Object Reference") (NormalImpulse :type "Vector Structure") (Hit :type "HitResult Structure (by ref)"))
  (`KismetSystemLibrary.PrintString` (`KismetSystemLibrary.GetObjectName` OtherActor)))

(fn `UserConstructionScript`)